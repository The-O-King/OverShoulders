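; VR pawn that reads motion controller triggers and grips and handles left-hand grabbing.
; Trigger axes and grip states are stored in variables, which this graph never reads.
; While InGripRange is true, left grip attaches every InteractActor_Static_BP in the level, not just a nearby one, to MeshL's GripSocket, keeping world position.
; Releasing left grip detaches them; right grip only sets its flag.
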(event EventBeginPlay)

(event Collision|EventActorBeginOverlap
  (params (OtherActor :type Actor%20Object%20Reference)))

(event EventTick
  (params (DeltaSeconds :type Float%20%28single-precision%29)))

(event Input|KeyboardEvents|MotionControllerRightTriggerAxis
  (params (AxisValue :type Float%20%28single-precision%29))
  (Variables|Default|SetrightTrigger AxisValue))

(event Input|KeyboardEvents|MotionControllerLeftTriggerAxis
  (params (AxisValue :type Float%20%28single-precision%29))
  (Variables|Default|SetleftTrigger AxisValue))

(event Input|KeyboardEvents|MotionControllerRightGrip1
  (params (Key :type Key%20Structure :default "AnyKey"))
  (:Pressed
    (Variables|Default|SetrightGrip true))
  (:Released
    (Variables|Default|SetrightGrip false)))

(event Input|KeyboardEvents|MotionControllerLeftGrip1
  (params (Key :type Key%20Structure :default "AnyKey"))
  (:Pressed
    (Variables|Default|SetleftGrip true)
    (if (Variables|Default|GetinGripRange)
      (bind _outactors (Actor|GetAllActorsOfClass "/Game/Blueprints/InteractActor_Static_BP.InteractActor_Static_BP_C"))
      (Class|Actor|AttachRootComponentto _outactors (Variables|Default|GetMeshL) "GripSocket" "KeepWorldPosition" true)))
  (:Released
    (Variables|Default|SetleftGrip false)
    (Class|Actor|DetachRootComponentfromParent _outactors true)))

(fn ConstructionScript)