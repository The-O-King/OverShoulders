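; A VR pawn Blueprint in the Tests folder that tracks motion controller grip and trigger input for both hands.
; Grip button presses and releases set left and right grip booleans.
; Trigger axis events store each hand's analog value and display it on that hand's pressure text component.
; The construction script is empty.
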(event Input|KeyboardEvents|MotionControllerLeftTriggerAxis
  (params (AxisValue :type Float%20%28single-precision%29))
  ;[1 1 1] Controls trigger inputs and displays pressure values
  (bind _output_get (Variables|Default|SetLeftTrigger AxisValue))
  (Rendering|Components|TextRender|SetText (Variables|Default|GetHand_L_Pressure) (Utilities|Text|ToText(Float) _output_get "HalfToEven")))

(event Input|KeyboardEvents|MotionControllerRightTriggerAxis
  (params (AxisValue :type Float%20%28single-precision%29))
  ;[1 1 1] Controls trigger inputs and displays pressure values
  (bind _output_get (Variables|Default|SetRightTrigger AxisValue))
  (Rendering|Components|TextRender|SetText (Variables|Default|GetHand_R_Pressure) (Utilities|Text|ToText(Float) _output_get "HalfToEven")))

(event Input|KeyboardEvents|MotionControllerLeftGrip1
  (params (Key :type Key%20Structure :default "AnyKey"))
  ;[1 1 1] Controls grip button inputs
  (:Pressed
    (Variables|Default|SetLeftGrip true))
  (:Released
    (Variables|Default|SetLeftGrip false)))

(event Input|KeyboardEvents|MotionControllerRightGrip1
  (params (Key :type Key%20Structure :default "AnyKey"))
  ;[1 1 1] Controls grip button inputs
  (:Pressed
    (Variables|Default|SetRightGrip true))
  (:Released
    (Variables|Default|SetRightGrip false)))

(fn ConstructionScript)