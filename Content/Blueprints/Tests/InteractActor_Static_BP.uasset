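; Test interactable static-mesh actor that tracks whether a VR_Pawn is within grip range.
; Begin and end overlap with a VR_Pawn set the pawn's InGripRange flag and store its inverse in Overlapped.
; Tick applies Overlapped to the mesh's physics simulation every frame, so despite the name, physics turns off when the pawn enters and on when it leaves.
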(event EventBeginPlay)

(event Collision|EventActorEndOverlap
  (params (OtherActor :type Actor%20Object%20Reference))
  (bind _asvr_pawn (Utilities|Casting|CastToVR_Pawn OtherActor))
  (bind _output_get (Variables|/Game/Blueprints/VR_Pawn.VR_Pawn_C|SetinGripRange _asvr_pawn false))
  (Variables|Default|SetOverlapped (not _output_get)))

(event EventTick
  (params (DeltaSeconds :type Float%20%28single-precision%29))
  (Physics|SetSimulatePhysics (Variables|Default|GetStaticMesh) (Variables|Default|GetOverlapped)))

(event Collision|EventActorBeginOverlap
  (params (OtherActor :type Actor%20Object%20Reference))
  (bind _asvr_pawn (Utilities|Casting|CastToVR_Pawn OtherActor))
  (bind _output_get (Variables|/Game/Blueprints/VR_Pawn.VR_Pawn_C|SetinGripRange _asvr_pawn true))
  (Variables|Default|SetOverlapped (not _output_get)))

(fn ConstructionScript)